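; BP_FXLooper is a preview-content actor that replays a particle effect on a loop at its own location and rotation.
; On BeginPlay it waits for InitialDelay, fires the template emitter once, then starts a looping timer at LoopTime intervals.
; Each firing deactivates the previous emitter, spawns a new one, then destroys the old component and stores the new reference.
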(event `self.ReceiveBeginPlay`
  ;[1 1 1] Panda Studios -- Set template \\ after initial delay on loop activate FX
  (`KismetSystemLibrary.Delay` (`self.InitialDelay`))
  (`self.FireFX`)
  (`KismetSystemLibrary.K2_SetTimerDelegate` (delegate `FireFX`) (`self.LoopTime`) true))

(event `FireFX`
  (bind _spawnedfx (`self.SpawnedFX`))
  (bind _spawnedfx_2 (`self.SpawnedFX`))
  ;[1 1 1] Panda Studios -- Set template \\ after initial delay on loop activate FX
  (`/Engine/EditorBlueprintResources/StandardMacros.IsValid` _spawnedfx_2
    (:`Is Valid`
      (`ActorComponent.Deactivate` _spawnedfx_2))
    (:`Is Not Valid`
      _))
  (bind _returnvalue (`GameplayStatics.SpawnEmitterAtLocation` (`self.Template`) (`self.K2_GetActorLocation`) (`self.K2_GetActorRotation`)))
  (`/Engine/EditorBlueprintResources/StandardMacros.IsValid` _spawnedfx
    (:`Is Valid`
      (`ActorComponent.K2_DestroyComponent` _spawnedfx))
    (:`Is Not Valid`
      _))
  (set `self.SpawnedFX` _returnvalue))

(fn `UserConstructionScript`)