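; A simple actor spawner from the PewPewPack preview content that spawns a configurable actor class on a repeating timer.
; After an initial delay on BeginPlay, a looping timer fires the spawn event at the SpawnTime interval.
; Each tick of the timer spawns the actor at the spawner's transform and attaches a muzzle particle effect to its Arrow component.
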(event `self.ReceiveBeginPlay`
  ;[1 1 1] Simple Actor Spawner
  (`KismetSystemLibrary.Delay` (`self.Innit Delay`))
  (`KismetSystemLibrary.K2_SetTimerDelegate` (delegate `Spawning`) (`self.SpawnTime`) true))

(event `Spawning`
  ;[1 1 1] Simple Actor Spawner
  (`|SpawnActorFromClass` (`self.SpawnActor`) (`self.GetTransform`) "Undefined" "OverrideRootScale")
  (`GameplayStatics.SpawnEmitterAttached` (`self.Muzzle`) (`self.Arrow`)))

(fn `UserConstructionScript`)