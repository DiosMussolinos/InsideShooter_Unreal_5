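; Base projectile actor for the PewPewPack preview content, with configurable muzzle, flight and impact particles and optional sounds.
; On BeginPlay it spawns the muzzle effect, sets local-space velocity and starts the projectile sound after a short delay.
; On hit it spawns the impact effect, fades flight audio, plays impact sound and destroys itself after a delay.
; Hueshifter applies hue and emissive strength to each effect through dynamic material instances.
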(event `self.ReceiveBeginPlay`
  (bind _sound_projectile_cue (`self.Sound_Projectile_Cue`))
  ;[1 1 1] Spawn emitter, set speed
  (`self.Hueshifter` (`self.Flying_Particle`))
  (bind _returnvalue (`GameplayStatics.SpawnEmitterAtLocation` (`self.Muzzle_Particle`) (`self.K2_GetActorLocation`) (`self.K2_GetActorRotation`)))
  (`self.Hueshifter` _returnvalue)
  (`ProjectileMovementComponent.SetVelocityInLocalSpace` (`self.ProjectileMovement`) (`self.Speed`))
  (`KismetSystemLibrary.Delay` 0.1)
  (if (`self.Play Sounds`)
    (`AudioComponent.SetSound` _sound_projectile_cue (`self.ProjectileCue`))
    (`AudioComponent.Play` _sound_projectile_cue 0.0)))

(event `self.ReceiveHit`
  (params (MyComp :type "PrimitiveComponent Object Reference") (Other :type "Actor Object Reference") (OtherComp :type "PrimitiveComponent Object Reference") (bSelfMoved :type Boolean) (HitLocation :type "Vector Structure") (HitNormal :type "Vector Structure") (NormalImpulse :type "Vector Structure") (Hit :type "HitResult Structure (by ref)"))
  (bind _sound_projectile_cue (`self.Sound_Projectile_Cue`))
  ;[1 1 1] On projectile hit
  (set `self.bHit` true)
  (bind _returnvalue (`GameplayStatics.SpawnEmitterAtLocation` (`self.Impact_Particle`) (`self.K2_GetActorLocation`) (`self.K2_GetActorRotation`)))
  (`self.Hueshifter` _returnvalue)
  (`ActorComponent.Deactivate` (`self.Flying_Particle`))
  (`/Engine/EditorBlueprintResources/StandardMacros.IsValid` _sound_projectile_cue
    (:`Is Valid`
      (`AudioComponent.FadeOut` _sound_projectile_cue 0.5 0.0)
      (if (`self.Play Sounds`)
        (`AudioComponent.SetSound` (`self.Sound_Impact_Cue`) (`self.ImpactCue`))
        (`AudioComponent.Play` (`self.Sound_Impact_Cue`) 0.0))
      (`KismetSystemLibrary.Delay` 1.0)
      (`ActorComponent.K2_DestroyComponent` (`self.Flying_Particle`))
      (`self.K2_DestroyActor`))))

(fn `Hueshifter`
  (params (HueShift :type "PrimitiveComponent Object Reference"))
  (for _index (range (`PrimitiveComponent.GetNumMaterials` HueShift))
    (bind _returnvalue (`PrimitiveComponent.CreateDynamicMaterialInstance` HueShift _index (`PrimitiveComponent.GetMaterial` HueShift _index)))
    (`MaterialInstanceDynamic.SetScalarParameterValue` _returnvalue "Hueshift" (`self.HueShift`))
    (`MaterialInstanceDynamic.SetScalarParameterValue` _returnvalue "EmissiveSTR" (`self.EmissiveSTR`))))

(fn `UserConstructionScript`
  (bind _flying_particle (`self.Flying_Particle`))
  (`ParticleSystemComponent.SetTemplate` _flying_particle (`self.Moving_Projectile`))
  (`self.Hueshifter` _flying_particle))